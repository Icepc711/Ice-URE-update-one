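; Base player character Blueprint that handles weapon acquisition, montage-driven switching and weapon animation lookup.
; After a short BeginPlay delay it spawns BPWeaponBase, attaches it to the mesh at the class-default socket and starts a switch.
; Switching stores a pending weapon and plays a montage; a hand-down notify event makes it current and calls WeaponInInventory on it.
; GetActiveWeaponAnim exposes its idle/walk animations; damage is only printed.
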(event `AcquireNewWeapon`
  (params (WeaponClass :type "/Game/blueprint/WeaponBease/BP-WeaponBase Class Reference"))
  (bind _equipsocketname (defaults `Object` WeaponClass))
  (bind _returnvalue (`|SpawnActorFromClass` WeaponClass (`SceneComponent.GetSocketTransform` (`self.Mesh`) _equipsocketname "RTS_World") "Undefined" "MultiplyWithRoot" self self))
  (`/Game/blueprint/WeaponBease/BP-WeaponBase.WeaponInInventory` _returnvalue)
  (`self.K2_AttachToComponent` _returnvalue (`self.Mesh`) _equipsocketname "SnapToTarget" "SnapToTarget" "KeepRelative" true)
  (`self.SwichActiveWeaponTo` _returnvalue))

(event `self.ReceiveBeginPlay`
  (`KismetSystemLibrary.Delay` 0.2)
  (`self.AcquireNewWeapon` "/Game/blueprint/WeaponBease/BP-WeaponBase.BP-WeaponBase_C"))

(event `SwichActiveWeaponTo`
  (params (NewActiveWeapon :type "/Game/blueprint/WeaponBease/BP-WeaponBase Object Reference"))
  (set `self.PendingNextActiveWeap` NewActiveWeapon)
  (`|PlayMontage` (`self.Mesh`) "/Game/animation/ASM_WeaponSwtich.ASM_WeaponSwtich"))

(event `WeaponSwichHandDownNotify`
  (`|ExecutionSequence`
    (:`then_0`
      (`/Engine/EditorBlueprintResources/StandardMacros.IsValid` (`self.CurrentActiveWeapon`)))
    (:`then_1`
      (bind _output_get (set `self.CurrentActiveWeapon` (`self.PendingNextActiveWeap`)))
      (`/Game/blueprint/WeaponBease/BP-WeaponBase.WeaponInInventory` _output_get))))

(event `self.ReceiveAnyDamage`
  (params (Damage :type "Float (single-precision)") (DamageType :type "DamageType Object Reference") (InstigatedBy :type "Controller Object Reference") (DamageCauser :type "Actor Object Reference"))
  (`KismetSystemLibrary.PrintString` (`KismetStringLibrary.Conv_DoubleToString` Damage)))

(fn `GetActiveWeaponAnim`
  (returns (IdleAnim :type "AnimSequence Object Reference") (WalkAnim :type "AnimSequence Object Reference"))
  (bind _currentactiveweapon (`self.CurrentActiveWeapon`))
  (return (`/Game/blueprint/WeaponBease/BP-WeaponBase.IdleAnim` _currentactiveweapon) (`/Game/blueprint/WeaponBease/BP-WeaponBase.WalkAnim` _currentactiveweapon)))

(fn `UserConstructionScript`)
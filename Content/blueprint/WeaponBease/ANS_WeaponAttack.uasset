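; Anim notify state for weapon attack animations that sets the state of the character's active weapon.
; Both notify begin and notify end cast the mesh owner to BP_charactorBase and write WeaponState on its CurrentActiveWeapon.
; Both events assign the same enum value (NewEnumerator1), so the end of the window does not switch the weapon to a different state.
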(fn `Received_NotifyBegin`
  (params (MeshComp :type "SkeletalMeshComponent Object Reference") (Animation :type "AnimSequenceBase Object Reference") (TotalDuration :type "Float (single-precision)") (EventReference :type "AnimNotifyEventReference Structure (by ref)"))
  (returns (ReturnValue :type Boolean))
  (bind _asbp_charactor_base (cast `/Game/PlayerAsset/BP_charactorBase` (`ActorComponent.GetOwner` MeshComp)))
  (set `/Game/blueprint/WeaponBease/BP-WeaponBase.WeaponState` "NewEnumerator1" (`/Game/PlayerAsset/BP_charactorBase.CurrentActiveWeapon` _asbp_charactor_base))
  (return false))

(fn `Recived Notify End`
  (params (MeshComp :type "SkeletalMeshComponent Object Reference") (Animation :type "AnimSequenceBase Object Reference") (TotalDuration :type "Float (single-precision)" :default 0.0) (EventReference :type "AnimNotifyEventReference Structure (by ref)"))
  (returns (ReturnValue :type Boolean))
  (bind _asbp_charactor_base (cast `/Game/PlayerAsset/BP_charactorBase` (`ActorComponent.GetOwner` MeshComp)))
  (set `/Game/blueprint/WeaponBease/BP-WeaponBase.WeaponState` "NewEnumerator1" (`/Game/PlayerAsset/BP_charactorBase.CurrentActiveWeapon` _asbp_charactor_base))
  (return false))
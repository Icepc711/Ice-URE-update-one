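; Grenade launcher weapon Blueprint that carries one loaded grenade and fires it along its owner's view direction.
; On BeginPlay it spawns a BP_Grenade and snaps it to the GernadeLaunchPoint socket on its static mesh.
; The CommitAttackAnimNotify event ignites the grenade with the owner's eye-view forward vector, then clears the reference; no reload happens here.
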(event `self.ReceiveBeginPlay`
  (`parent.ReceiveBeginPlay`)
  (`self.LoadGrenadeOnSpawn`))

(event `LoadGrenadeOnSpawn`
  (bind _returnvalue (`|SpawnActorFromClass` "/Game/blueprint/WeaponBease/BP_Grenade.BP_Grenade_C" (`SceneComponent.GetSocketTransform` (`self.StaticMesh`) (`self.GernadeLaunchPoint`) "RTS_World") "Undefined" "MultiplyWithRoot" self null))
  (bind _output_get (set `self.LoadedGrenade` _returnvalue))
  (`self.K2_AttachToComponent` _output_get (`self.StaticMesh`) (`self.GernadeLaunchPoint`) "SnapToTarget" "SnapToTarget" "SnapToTarget" true))

(event `self.CommitAttackAnimNotify`
  (`/Engine/EditorBlueprintResources/StandardMacros.IsValid` (`self.LoadedGrenade`)
    (:`Is Valid`
      (`/Game/blueprint/WeaponBease/BP_Grenade.Ignite` (`self.LoadedGrenade`) (`KismetMathLibrary.GetForwardVector` (`.OutRotation` (`self.GetActorEyesViewPoint` (`self.GetOwner`)))))
      (set `self.LoadedGrenade` null))))

(fn `UserConstructionScript`
  (`parent.UserConstructionScript`))